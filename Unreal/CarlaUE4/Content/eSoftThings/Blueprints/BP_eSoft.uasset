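; Actor that drives mirror displays and a central warning screen on a mesh, apparently a vehicle, from webcams and network feeds.
; A TCP image receiver streams into the right mirror material, while UDP listeners switch the warning material and set a mixed-mode flag.
; Tick polls the listeners and swaps mixed/virtual material maps when that flag changes.
; Left virtual mirror setup is disconnected, so both maps use the mixed left material.
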(event `self.ReceiveBeginPlay`
  (bind _left (`self.Left`))
  (bind _right (`self.Right`))
  (`parent.ReceiveBeginPlay`)
  (`MediaPlayer.OpenUrl` _left "vidcap://\\\\?\\usb#vid_1bcf&pid_2c99&mi_00#6&3038eb23&0&0000#{e5323777-f976-4f5b-9b55-b94699c46e44}\\global")
  (`MediaPlayer.OpenUrl` _right "vidcap://\\\\?\\usb#vid_1bcf&pid_2c99&mi_00#6&3038eb23&0&0000#{e5323777-f976-4f5b-9b55-b94699c46e44}\\global")
  (`MediaPlayer.Play` _left)
  (`MediaPlayer.Play` _right)
  (bind _returnvalue (`PrimitiveComponent.CreateDynamicMaterialInstance` (`self.Mesh`) 6 "/Game/eSoftThings/CarModel/CarMaterials/Central_Screen.Central_Screen" "None"))
  (bind _returnvalue_2 (`|GenericCreateObject` "/Game/eSoftThings/Blueprints/UDP/UDPMaterialSwitch.UDPMaterialSwitch_C" self _returnvalue))
  (`KismetArrayLibrary.Array_Add` (`self.UDPListeners`) _returnvalue_2)
  (`UDPListener.Init` _returnvalue_2 "String" 5583 32)
  (bind _returnvalue_3 (`|GenericCreateObject` "/Game/eSoftThings/Blueprints/UDP/UDPBoolSetter.UDPBoolSetter_C" self))
  (`KismetArrayLibrary.Array_Add` (`self.UDPListeners`) _returnvalue_3)
  (bind _output_get (set `self.MixedModeReceiver` _returnvalue_3))
  (`UDPListener.Init` _output_get "String" 5582 32)
  (bind _returnvalue_4 (`PrimitiveComponent.CreateDynamicMaterialInstance` (`self.Mesh`) 0 "/Game/eSoftThings/DynamicMaterials/Mat_Virtual_Right.Mat_Virtual_Right" "None"))
  (`BlueprintMapLibrary.Map_Add` (`self.Virtual_Materials`) 0 _returnvalue_4)
  (`BlueprintMapLibrary.Map_Add` (`self.Mixed_Materials`) 0 _returnvalue_4)
  (bind _returnvalue_5 (`|GenericCreateObject` "/Game/eSoftThings/Blueprints/UDP/TCPImageReceiver.TCPImageReceiver_C" self _returnvalue_4))
  (`KismetArrayLibrary.Array_Add` (`self.TCPListeners`) _returnvalue_5)
  (bind _returnvalue_6 (`TCPImageListener.SetImageSize` _returnvalue_5 1280 800 "PF_B8G8R8A8" 4))
  (`TCPImageListener.Init` _returnvalue_5 5580 _returnvalue_6)
  (`self.AddDynamicInstance` "/Game/eSoftThings/DynamicMaterials/Mat_Mixed_Left.Mat_Mixed_Left" (`self.Mixed_Materials`) 9)
  (`self.AddDynamicInstance` "/Game/eSoftThings/DynamicMaterials/Mat_Mixed_Left.Mat_Mixed_Left" (`self.Virtual_Materials`) 9))

(event `self.ReceiveTick`
  (params (DeltaSeconds :type "Float (single-precision)"))
  (bind _mixedmodereceiver (`self.MixedModeReceiver`))
  (bind _value (`/Game/eSoftThings/Blueprints/UDP/UDPBoolSetter.Value` _mixedmodereceiver))
  (`parent.ReceiveTick` DeltaSeconds)
  (for _array_element (`self.UDPListeners`)
    (`UDPListener.Tick` _array_element))
  (for _array_element_2 (`self.TCPListeners`)
    (`TCPImageListener.Tick` _array_element_2))
  (if (== _mixedmodereceiver null)
    _
    (elif (!= (`self.MixedModeLastValue`) _value)
      (bind _output_get (set `self.MixedModeLastValue` _value))
      (if _output_get
        (`self.SetMaterialsWithIndex` (`self.Mixed_Materials`))
        (else
          (`self.SetMaterialsWithIndex` (`self.Virtual_Materials`)))))))

(event `self.ReceiveEndPlay`
  (params (EndPlayReason :type "EEndPlayReason Enum" :default "Destroyed"))
  (for _array_element (`self.UDPListeners`)
    (`UDPListener.Stop` _array_element))
  (for _array_element_2 (`self.TCPListeners`)
    (`TCPImageListener.Stop` _array_element_2)
    (`KismetSystemLibrary.QuitGame` null "Quit" true)))

(fn `AddDynamicInstance`
  (params (`Base Material` :type "Material Object Reference") (Map :type "Map of Integer to MaterialInstanceDynamic Object Reference (by ref)") (MaterialIndex :type Integer))
  (bind _returnvalue (`PrimitiveComponent.CreateDynamicMaterialInstance` (`self.Mesh`) MaterialIndex `Base Material` "None"))
  (`BlueprintMapLibrary.Map_Add` Map MaterialIndex _returnvalue))

(fn `SetMaterialsWithIndex`
  (params (InputPin :type "Map of Integer to MaterialInstanceDynamic Object Reference (by ref)"))
  (bind _keys (`BlueprintMapLibrary.Map_Keys` InputPin))
  (for _array_element _keys
    (`PrimitiveComponent.SetMaterial` (`self.Mesh`) _array_element (`BlueprintMapLibrary.Map_Find` InputPin _array_element))))

(fn `UserConstructionScript`
  (`parent.UserConstructionScript`))